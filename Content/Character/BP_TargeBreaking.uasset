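; Breakable target actor that takes damage and shows its remaining endurance on a text render.
; On BeginPlay the authority rolls a random starting Endurance, and an OnRep function refreshes the displayed number, clamped at zero, when the value replicates.
; The Hit event subtracts damage until Endurance runs out, then sets Breaking to block further hits and swaps the static mesh to SM_Couch.
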(event `self.ReceiveBeginPlay`
  (`parent.ReceiveBeginPlay`)
  (`/Engine/EditorBlueprintResources/ActorMacros.Switch Has Authority`
    (:`Authority`
      (bind _output_get (set `self.Endurance` (`KismetMathLibrary.RandomIntegerInRange` 100 200))))
    (:`Remote`
      _))
  (`TextRenderComponent.K2_SetText` (`self.TextRender`) (`KismetTextLibrary.Conv_IntToText` _output_get)))

(event `/Game/Core/BPI_Hit.Hit`
  (params (Damage :type Integer))
  (if (not (`self.Breaking`))
    (bind _output_get (set `self.Endurance` (- (`self.Endurance`) Damage)))
    (if (== (`KismetMathLibrary.Max` _output_get) 0)
      (set `self.Breaking` true)
      (`StaticMeshComponent.SetStaticMesh` (`self.StaticMesh`) "/Game/StarterContent/Props/SM_Couch.SM_Couch"))))

(fn `OnRep_Endurance`
  (`TextRenderComponent.K2_SetText` (`self.TextRender`) (`KismetTextLibrary.Conv_IntToText` (`KismetMathLibrary.Max` (`self.Endurance`)))))

(fn `UserConstructionScript`
  (`parent.UserConstructionScript`))