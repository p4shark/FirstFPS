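; BP_HandActor is an interactable item that a BP_Character can pick up, swap and drop through its active inventory slot.
; Interract fills the slot, first moving any held item to this actor's transform and unbinding fire if it is a BP_Weapon.
; Attachment branches on network authority: first-person GripPoint on authority, body-mesh hand_r on remote.
; Drop detaches the item, places it ahead of the player and clears the slot.
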(event `/Game/Core/BPI_Interract.Interract`
  (params (Player :type "Actor Object Reference"))
  (bind _asbp_character (cast `/Game/Character/BP_Character` Player))
  (`/Engine/EditorBlueprintResources/StandardMacros.IsValid` (`self.GetActorInPlayerHand` _asbp_character)
    (:`Is Valid`
      (`self.SwapActorInHandAndNewActor` _asbp_character))
    (:`Is Not Valid`
      (`/Engine/EditorBlueprintResources/ActorMacros.Switch Has Authority`
        (:`Authority`
          (`self.K2_AttachToComponent` (`/Game/Character/BP_Character.FirstPersonMesh` _asbp_character) "GripPoint" "SnapToTarget" "SnapToTarget" "SnapToTarget"))
        (:`Remote`
          (`self.K2_AttachToComponent` (`Character.Mesh` _asbp_character) "hand_r" "SnapToTarget" "SnapToTarget" "SnapToTarget")))
      (`KismetArrayLibrary.Array_Set` (`/Game/Character/BP_Character.Inventory` _asbp_character) (`/Game/Character/BP_Character.ActiveSlot` _asbp_character) self))))

(event `/Game/Core/BPI_Interract.Drop`
  (params (Player :type "Actor Object Reference"))
  (bind _asbp_character (cast `/Game/Character/BP_Character` Player))
  (`self.K2_DetachFromActor` self "KeepRelative" "KeepRelative" "KeepRelative")
  (`self.K2_SetActorTransform` self (`KismetMathLibrary.MakeTransform` (+ (* (`KismetMathLibrary.Normal` (`self.GetActorForwardVector` _asbp_character)) 100.0) (`self.K2_GetActorLocation` _asbp_character))) false false)
  (`KismetArrayLibrary.Array_Set` (`/Game/Character/BP_Character.Inventory` _asbp_character) (`/Game/Character/BP_Character.ActiveSlot` _asbp_character)))

(fn `GetActorInPlayerHand`
  (params (Player :type "/Game/Character/BP_Character Object Reference"))
  (returns (`Actor in hand` :type "/Game/Core/Objects/BP_HandActor Object Reference"))
  (return (`|GetArrayItem` (`/Game/Character/BP_Character.Inventory` Player) (`/Game/Character/BP_Character.ActiveSlot` Player))))

(fn `SwapActorInHandAndNewActor`
  (params (Player :type "/Game/Character/BP_Character Object Reference"))
  (bind _actor_in_hand (`self.GetActorInPlayerHand` Player))
  (bind _asbp_weapon (cast `/Game/Core/Objects/Weapons/BP_Weapon` _actor_in_hand)
    (:`then`
      (`/Game/Core/Objects/Weapons/BP_Weapon.UnbindFire` _asbp_weapon))
    (:`CastFailed`
      _))
  (`self.K2_DetachFromActor` _actor_in_hand "KeepRelative" "KeepRelative" "KeepRelative")
  (`self.K2_SetActorTransform` _actor_in_hand (`self.GetTransform` self) false false)
  (`KismetArrayLibrary.Array_Set` (`/Game/Character/BP_Character.Inventory` Player) (`/Game/Character/BP_Character.ActiveSlot` Player) self)
  (`/Engine/EditorBlueprintResources/ActorMacros.Switch Has Authority`
    (:`Authority`
      (`self.K2_AttachToComponent` (`/Game/Character/BP_Character.FirstPersonMesh` Player) "GripPoint" "SnapToTarget" "SnapToTarget" "SnapToTarget"))
    (:`Remote`
      (`self.K2_AttachToComponent` (`Character.Mesh` Player) "hand_r" "SnapToTarget" "SnapToTarget" "SnapToTarget"))))

(fn `UserConstructionScript`)