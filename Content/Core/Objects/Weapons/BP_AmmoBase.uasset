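; Base ammo pickup that a player collects by interacting with it.
; Interact adds PackSize to the character's Ammunition map under AmmoType, updates the active-slot count if the held weapon uses that type, then destroys the pickup.
; The character reference's RepNotify calls ClientUpdate only on authority.
; ChangeAmmoFromPlayer does nothing, as its map-update and multicast logic is disconnected.
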(event `/Game/Core/BPI_Interract.Interract`
  (params (Player :type "Actor Object Reference"))
  (bind _asbp_character (cast `/Game/Character/BP_Character` Player))
  (set `self.FirstPersonCharacterReference` _asbp_character)
  (bind _ammunition (`/Game/Character/BP_Character.Ammunition` _asbp_character))
  (bind (_value _returnvalue) (`BlueprintMapLibrary.Map_Find` _ammunition (`self.AmmoType`)))
  (if _returnvalue
    (bind _output_get (set `self.LocalAmmo` _value))
    (`BlueprintMapLibrary.Map_Remove` _ammunition (`self.AmmoType`))
    (bind _ammunition_2 (`/Game/Character/BP_Character.Ammunition` _asbp_character))
    (bind _returnvalue_2 (+ _output_get (`self.PackSize`)))
    (`BlueprintMapLibrary.Map_Add` _ammunition_2 (`self.AmmoType`) _returnvalue_2)
    (if (`self.CheckAmmoType`)
      (set `/Game/Character/BP_Character.AmmoInActoveSlot` _returnvalue_2 (`self.FirstPersonCharacterReference`)))
    (`self.K2_DestroyActor`)
    (else
      (`BlueprintMapLibrary.Map_Add` _ammunition_2 (`self.AmmoType`) (`self.PackSize`))
      (if (`self.CheckAmmoType`)
        (set `/Game/Character/BP_Character.AmmoInActoveSlot` (`self.PackSize`) (`self.FirstPersonCharacterReference`)))
      (`self.K2_DestroyActor`))))

(fn `ChangeAmmoFromPlayer`
  (params (NewAmmo :type Integer) (NewBullenInCllip :type Integer)))

(fn `CheckAmmoType`
  (returns (ReturnValue :type Boolean))
  (bind _asbp_weapon (cast `/Game/Core/Objects/Weapons/BP_Weapon` (`/Game/Character/BP_Character.GetActorInPlayerHand` (`self.FirstPersonCharacterReference`))))
  (return (== (`/Game/Core/Objects/Weapons/BP_Weapon.AmmoType` _asbp_weapon) (`self.AmmoType`))))

(fn `OnRep_FirstPersonCharacterReference`
  (`/Engine/EditorBlueprintResources/ActorMacros.Switch Has Authority`
    (:`Authority`
      (`/Game/Character/BP_Character.ClientUpdate` (`self.FirstPersonCharacterReference`)))))

(fn `UserConstructionScript`)